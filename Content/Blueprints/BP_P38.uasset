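; BP_P38 is a P-38 aircraft Blueprint that flies forward continuously and spins its two propellers.
; Each Tick offsets the actor along its local X axis by MovementSpeed scaled by delta time.
; RotatePropeller adds a frame-rate-independent relative roll to the Left and Right propellers using PropellerRotationSpeed.
; Pitch and Roll input axis events exist but are empty, so the plane has no steering.
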(event `self.ReceiveTick`
  (params (DeltaSeconds :type "Float (single-precision)"))
  ;[1 1 1] 앞으로 이동
  (`self.K2_AddActorLocalOffset` (`KismetMathLibrary.MakeVector` (* (`GameplayStatics.GetWorldDeltaSeconds`) (`self.MovementSpeed`))))
  ;[1 1 1] 왼쪽 프로펠러 회전
  (`self.RotatePropeller` (`self.Left`))
  ;[1 1 1] 오른쪽 프로펠러 회전
  (`self.RotatePropeller` (`self.Right`)))

(event `InputAxis|Pitch`
  (params (AxisValue :type "Float (single-precision)")))

(event `InputAxis|Roll`
  (params (AxisValue :type "Float (single-precision)")))

(fn `RotatePropeller`
  (params (Where :type "StaticMeshComponent Object Reference"))
  (`SceneComponent.K2_AddRelativeRotation` Where (`KismetMathLibrary.MakeRotator` (* (`GameplayStatics.GetWorldDeltaSeconds`) (`self.PropellerRotationSpeed`))) false false))

(fn `UserConstructionScript`)